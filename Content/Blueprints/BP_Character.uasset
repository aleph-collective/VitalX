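; Character Blueprint that exposes health and energy readouts from its Vitals object.
; Raw fetch functions return the current value divided by 100, plus the unscaled native value, which suggests fixed-point storage.
; Ratio functions divide that scaled value by the equally scaled maximum to give a current-to-max fraction.
; The event graph and construction script hold no logic.
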(fn `FetchEnergyRatio`
  (returns (ReturnValue :type "Float (double-precision)"))
  (bind _returnvalue (`self.FetchEnergyRaw`))
  (return (/ _returnvalue (/ (`KismetMathLibrary.Conv_IntToDouble` (`Vitals.MaxEnergy` (`self.Vitals`))) 100.0))))

(fn `FetchEnergyRaw`
  (returns (ReturnValue :type "Float (double-precision)") (ReturnaNativeValue :type Integer))
  (bind _returnvalue (`Vitals.GetEnergy` (`self.Vitals`)))
  (return (/ (`KismetMathLibrary.Conv_IntToDouble` _returnvalue) 100.0) _returnvalue))

(fn `FetchHealthRatio`
  (returns (ReturnValue :type "Float (double-precision)"))
  (bind _returnvalue (`self.FetchHealthRaw`))
  (return (/ _returnvalue (/ (`KismetMathLibrary.Conv_IntToDouble` (`Vitals.MaxHealth` (`self.Vitals`))) 100.0))))

(fn `FetchHealthRaw`
  (returns (ReturnValue :type "Float (double-precision)") (ReturnNativeValue :type Integer))
  (bind _returnvalue (`Vitals.GetHealth` (`self.Vitals`)))
  (return (/ (`KismetMathLibrary.Conv_IntToDouble` _returnvalue) 100.0) _returnvalue))

(fn `UserConstructionScript`)